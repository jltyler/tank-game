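; Test projectile Blueprint with debug helpers that visualise the motion of its ProjectileMovement component.
; DrawTrajectory steps through a time span at a given interval, drawing spheres at positions predicted from current location, velocity and gravity by the constant-acceleration kinematic equation.
; DrawVelocity draws a short-lived line from the actor along its current velocity vector.
; The event graph and construction script are empty, so neither helper is called within this Blueprint.
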(event Collision|EventActorBeginOverlap
  (params (OtherActor :type Actor%20Object%20Reference)))

(event EventTick
  (params (DeltaSeconds :type Float%20%28single-precision%29)))

(fn ConstructionScript)

(fn DrawTrajectory
  (params (Time :type Float%20%28single-precision%29) (Interval :type Float%20%28single-precision%29))
  (bind _projectilemovement (Variables|Default|GetProjectileMovement))
  (bind _velocity (Variables|/Script/Engine.MovementComponent|GetVelocity _projectilemovement))
  (bind (_x _y _z) (Math|Vector|BreakVector _velocity))
  (for _index (range 1 (Math|Float|Truncate (/ Time Interval)))
    (Rendering|Debug|DrawDebugSphere (+ (Math|Vector|MakeVector (* _x (Math|Float|MakeLiteralFloat (* _index Interval))) (* _y (Math|Float|MakeLiteralFloat (* _index Interval))) (+ (* _z (Math|Float|MakeLiteralFloat (* _index Interval))) (* (* (Components|Movement|GetGravityZ _projectilemovement) 0.5) (Math|Float|Square (Math|Float|MakeLiteralFloat (* _index Interval)))))) (Transformation|GetActorLocation)) 1e+02 12 "(R=0.000000,G=1.000000,B=0.989507,A=1.000000)" Time 2e+01)))

(fn DrawVelocity
  (bind _returnvalue (Transformation|GetActorLocation))
  (Rendering|Debug|DrawDebugLine _returnvalue (+ _returnvalue (Variables|/Script/Engine.MovementComponent|GetVelocity (Variables|Default|GetProjectileMovement))) "(R=0.799486,G=0.000000,B=1.000000,A=1.000000)" 1.0 2e+01))