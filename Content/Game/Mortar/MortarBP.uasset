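; Mortar Blueprint that aims at a given location and fires projectiles through an Aiming component.
; On BeginPlay it passes its inner barrel, turret and fire point to Aiming, and falls back to a test projectile class when none is set.
; AimAt, StartFiring and StopFiring events simply forward to the Aiming component, which holds the aiming and firing logic.
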(event EventBeginPlay
  (bind _aiming (Variables|Default|GetAiming))
  (Class|AimingComponent|Initialize (Variables|Default|GetAiming) (Variables|Default|GetBarrelInner) (Variables|Default|GetTurret) (Variables|Default|GetFirePoint))
  ;[1 1 1] Set WeaponProjectile if invalid
  (if (not (Utilities|IsValidClass (Variables|/Script/TankArruz.AimingComponent|GetWeaponProjectile _aiming)))
    (Variables|/Script/TankArruz.AimingComponent|SetWeaponProjectile _aiming "/Game/Game/Projectile/TestProjectileBP.TestProjectileBP_C")))

(event EventStartFiring
  ;[1 1 1] Firing Events
  (Class|AimingComponent|StartFiring (Variables|Default|GetAiming)))

(event EventStopFiring
  ;[1 1 1] Firing Events
  (Class|AimingComponent|StopFiring (Variables|Default|GetAiming)))

(event EventAimat
  (params (AimLocation :type Vector%20%28by%20ref%29 :default "0, 0, 0"))
  ;[1 1 1] AimAt Event
  (Class|AimingComponent|AimatLocation (Variables|Default|GetAiming) AimLocation))

(fn ConstructionScript)