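; Player controller that creates the player's HUD and an in-game menu.
; On BeginPlay it adds the PlayerUI widget to the viewport, then adds the IngameMenu widget hidden and keeps a reference to it.
; Pressing Cancel while the menu is not visible shows it, enables the mouse cursor and switches input to UI-only focused on the menu.
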(event EventBeginPlay
  (Utilities|FlowControl|Sequence
    (:then_0
      (bind _returnvalue (UserInterface|CreateWidget "/Game/Blueprints/PlayerUI.PlayerUI_C"))
      (UserInterface|Viewport|AddtoViewport _returnvalue 0))
    (:then_1
      (bind _returnvalue_2 (UserInterface|CreateWidget "/Game/Blueprints/IngameMenu.IngameMenu_C"))
      (bind _output_get (Variables|Default|SetIngameMenu _returnvalue_2))
      (UserInterface|Viewport|AddtoViewport _output_get 0)
      (Widget|SetVisibility _output_get "Hidden"))))

(event EventTick
  (params (DeltaSeconds :type Float%20%28single-precision%29)))

(event Input|ActionEvents|InputActionCancel
  (params (Key :type Key%20Structure))
  (bind _ingamemenu (Variables|Default|GetIngameMenu))
  (:Pressed
    (if (not (Widget|IsVisible _ingamemenu))
      (Widget|SetVisibility _ingamemenu "Visible")
      (Variables|Default|SetbShowMouseCursor true)
      (Input|SetInputModeUIOnly self _ingamemenu "DoNotLock"))))

(fn ConstructionScript)