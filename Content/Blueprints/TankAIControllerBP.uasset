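; AI controller Blueprint for enemy tanks that handles auto-firing at the player and recovery from flipping.
; On possessing a tank it enables refire on the AimingComponent, starts looping timers, and sets a pursue distance for mortar pawns.
; A range check fires while aim is locked and the player is within twice that distance.
; A slower check lifts upside-down tanks and resets their roll.
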(event Custom|TankFireWeapon
  ;[1 1 1] Fire with random intervals
)

(event Custom|CheckRange
  (bind _controlledtank (Variables|Default|GetControlledTank))
  ;[1 1 1] If within PursueDistance * 2 to player AND AimingComponent is LockedOn then fire at player
  (if (and (Utilities|Enum|Equal(Enum) (Class|AimingComponent|GetFiringStatus (Actor|GetComponentbyClass _controlledtank "/Script/TankArruz.AimingComponent")) "LockedOn") (<= (Math|Vector|VectorLength (- (Transformation|GetActorLocation _controlledtank) (Transformation|GetActorLocation (Variables|Default|GetPlayerTank)))) (* (Variables|Default|GetPursueDistance) 2.0)))
    (Class|Tank|StartFiring _controlledtank)
    (else
      (Class|Tank|StopFiring _controlledtank))))

(event Custom|DEBUG
  (bind _controlledtank (Variables|Default|GetControlledTank))
  (bind _returnvalue (Transformation|GetActorLocation _controlledtank))
  ;[1 1 1] Draw Aim Vector Line
  (Rendering|Debug|DrawDebugLine _returnvalue (+ _returnvalue (+ (Class|AimingComponent|GetAimVector (Actor|GetComponentbyClass _controlledtank "/Script/TankArruz.AimingComponent")) 1e+03)) "(R=0.744792,G=0.000000,B=0.527691,A=1.000000)" 2.0 1e+01))

(event Custom|CheckFlipOver
  (bind _controlledtank (Variables|Default|GetControlledTank))
  (bind _returnvalue (Transformation|GetActorRotation _controlledtank))
  (if (> (Math|Vector|DotProduct (Math|Vector|MakeVector 0.0 0.0 -1.0) (Transformation|GetActorUpVector (Variables|Default|GetControlledTank))) 0.0)
    (Transformation|SetActorLocationAndRotation _controlledtank (+ (Transformation|GetActorLocation _controlledtank) (Math|Vector|MakeVector 0.0 0.0 1e+02)) (Math|Rotator|MakeRotator 0.0 (.pitch _returnvalue) (.yaw _returnvalue)) false true)))

(event EventBeginPlay)

(event EventNewTankPossessed
  (params (NewTank :type Tank%20Object%20Reference))
  ;[1 1 1] Turn on auto fire
  (Variables|/Script/TankArruz.AimingComponent|SetRefire (Actor|GetComponentbyClass (Variables|Default|GetControlledTank) "/Script/TankArruz.AimingComponent") true)
  (Utilities|Time|SetTimerbyEvent (delegate Custom|CheckRange) 1.0 true)
  (Utilities|Time|SetTimerbyEvent 0 2.0 true)
  (Utilities|Time|SetTimerbyEvent (delegate Custom|CheckFlipOver) 2e+01 true)
  (Utilities|Casting|CastToMortarBP (Pawn|GetControlledPawn))
  (Variables|Default|SetPursueDistance 4e+04))

(fn ConstructionScript)