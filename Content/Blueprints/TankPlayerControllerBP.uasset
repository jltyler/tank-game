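; Player controller for a tank that handles firing input and creates the player's UI and hidden in-game menu.
; On BeginPlay it passes the TankBP aiming component to the UI widget, which plays a reload fade when Fire is pressed before reloading finishes.
; Fire starts and stops tank firing, and Cancel is forwarded to the menu.
; A looping timer uses an up-vector dot product to detect a flipped tank, then lifts and rights it.
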(event Custom|CheckFlipOver
  (bind _controlledtank (Variables|Default|GetControlledTank))
  (bind _returnvalue (Transformation|GetActorRotation _controlledtank))
  ;[1 1 1] Flip ControlledTank if upside down
  (if (> (Math|Vector|DotProduct (Math|Vector|MakeVector 0.0 0.0 -1.0) (Transformation|GetActorUpVector (Variables|Default|GetControlledTank))) 0.0)
    (Transformation|SetActorLocationAndRotation _controlledtank (+ (Transformation|GetActorLocation _controlledtank) (Math|Vector|MakeVector 0.0 0.0 1e+02)) (Math|Rotator|MakeRotator 0.0 (.pitch _returnvalue) (.yaw _returnvalue)) false true)))

(event EventBeginPlay
  (Utilities|FlowControl|Sequence
    (:then_0
      ;[1 1 1] Get TankBP AimingComponent
      (bind _astank_bp (Utilities|Casting|CastToTankBP (Pawn|GetControlledPawn)))
      (Variables|Default|SetTankAimingComponent (Variables|/Game/Game/Tank/TankBP.TankBP_C|GetAiming _astank_bp)))
    (:then_1
      ;[1 1 1] Setup Player UI Widget
      (bind _returnvalue (UserInterface|CreateWidget "/Game/Blueprints/PlayerUI.PlayerUI_C"))
      (Variables|/Game/Blueprints/PlayerUI.PlayerUI_C|SetPlayerAimingComponent _returnvalue (Variables|Default|GetTankAimingComponent))
      (UserInterface|Viewport|AddtoViewport _returnvalue 0))
    (:then_2
      ;[1 1 1] Setup Ingame Menu Widget
      (bind _returnvalue_2 (UserInterface|CreateWidget "/Game/Blueprints/IngameMenu.IngameMenu_C"))
      (bind _output_get (Variables|Default|SetIngameMenu _returnvalue_2))
      (UserInterface|Viewport|AddtoViewport _output_get 0)
      (Widget|SetVisibility _output_get "Hidden"))
    (:then_3
      (Utilities|Time|SetTimerbyEvent (delegate Custom|CheckFlipOver) 2e+01 true))))

(event Input|ActionEvents|InputActionCancel
  (params (Key :type Key%20Structure))
  ;[1 1 1] Bind Cancel to Menu Cancel
  (:Pressed
    (Default|OnCancel (stale EventBeginPlay _output_get))))

(event Input|ActionEvents|InputActionFire
  (params (Key :type Key%20Structure))
  (bind _controlledtank (Variables|Default|GetControlledTank))
  ;[1 1 1] Reload flashage
  (:Pressed
    (if (Variables|/Script/TankArruz.AimingComponent|GetReloaded (Variables|Default|GetTankAimingComponent))
      _
      (else
        (UserInterface|Animation|PlayAnimation (stale EventBeginPlay _returnvalue) (Variables|/Game/Blueprints/PlayerUI.PlayerUI_C|GetReload%20fade (stale EventBeginPlay _returnvalue)) 0.0 1 "Forward" 1.0)))
    (Class|Tank|StartFiring _controlledtank))
  (:Released
    (Class|Tank|StopFiring _controlledtank)))

(fn ConstructionScript)